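; BP_Monster is an input-driven monster pawn that moves along its facing and turns with the movement axes.
; MoveForward adds movement along the yaw-only control rotation, scaled by MoveSpeed, with BackSpeed also applied when reversing.
; MoveRight adds controller yaw, using BaseTurnRate and frame time for positive input but negated BackSpeed without frame time for negative input.
; The construction script only calls its parent.
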(event `InputAxis|MoveForward` :overrideparent false
  (params (AxisValue :type "Float (single-precision)"))
  (`self.AddMovementInput` (`KismetMathLibrary.GetForwardVector` (`KismetMathLibrary.MakeRotator` 0.0 0.0 (.yaw (`self.GetControlRotation`)))) (* (select `bool` (>= AxisValue 0.0) :`false` (* AxisValue (`self.BackSpeed`)) :`true` AxisValue) (`self.MoveSpeed`))))

(event `InputAxis|MoveRight` :overrideparent false
  (params (AxisValue :type "Float (single-precision)"))
  (`self.AddControllerYawInput` (select `bool` (>= (stale `InputAxis|MoveForward` AxisValue) 0.0) :`false` (* AxisValue (* (`self.BackSpeed`) -1.0)) :`true` (* AxisValue (`self.BaseTurnRate`) (`GameplayStatics.GetWorldDeltaSeconds`)))))

(fn `UserConstructionScript`
  (`parent.UserConstructionScript`))