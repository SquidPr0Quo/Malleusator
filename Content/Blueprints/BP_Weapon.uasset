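; BP_Weapon is a melee-style weapon, owned by its parent actor, that damages BP_Player characters.
; When its sphere overlaps a player capsule of a different class from the owner, a delayed-loop macro repeats short line traces.
; The loop has no end-overlap exit and runs until a trace strikes that player's mesh.
; The hit calls GotHit with a direction and base damage scaled by the wielder's Brawn.
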(event `self.Sphere.OnComponentBeginOverlap`
  (params (OverlappedComponent :type "PrimitiveComponent Object Reference") (OtherActor :type "Actor Object Reference") (OtherComp :type "PrimitiveComponent Object Reference") (OtherBodyIndex :type Integer) (bFromSweep :type Boolean) (SweepResult :type "HitResult Structure (by ref)"))
  (bind _defaultsceneroot (`self.DefaultSceneRoot`))
  (bind _defaultsceneroot_2 (`self.DefaultSceneRoot`))
  (bind _returnvalue (`SceneComponent.K2_GetComponentLocation` _defaultsceneroot_2))
  (bind _returnvalue_2 (`SceneComponent.K2_GetComponentLocation` _defaultsceneroot))
  (if (not (== (`GameplayStatics.GetObjectClass` OtherActor) (`GameplayStatics.GetObjectClass` (`self.weaponParent`))))
    (bind _asbp_player (cast `/Game/Blueprints/BP_Player` OtherActor))
    (set `self.TargetMesh` (`Character.Mesh` _asbp_player))
    (set `self.hitTarget` _asbp_player)
    (if (== (`Character.CapsuleComponent` _asbp_player) OtherComp)
      (`self.WhileLoopWidthDelay` (not (`self.didHit`)) 0.1
        (:`Body`
          (bind (_outhit _returnvalue_3) (`KismetSystemLibrary.LineTraceSingle` _returnvalue (- _returnvalue (* (`KismetMathLibrary.GetForwardVector` (`SceneComponent.K2_GetComponentRotation` _defaultsceneroot_2)) 5.0)) "TraceTypeQuery1" true (`|MakeArray` (`self.weaponParent`)) "ForDuration" true (struct :`R` 1.0 :`A` 1.0) (struct :`G` 1.0 :`A` 1.0) 0.1))
          (if _returnvalue_3
            (if (== (`.HitComponent` (`GameplayStatics.BreakHitResult` _outhit)) (`self.TargetMesh`))
              (set `self.didHit` true)
              (bind _asbp_player_2 (cast `/Game/Blueprints/BP_Player` (`self.weaponParent`)))
              (`/Game/Blueprints/BP_Player.GotHit` (`self.hitTarget`) (- _returnvalue_2 (+ _returnvalue_2 (`KismetMathLibrary.GetForwardVector` (`SceneComponent.K2_GetComponentRotation` _defaultsceneroot)))) (* (`self.baseDamage`) (`/Game/Blueprints/BP_Player.Brawn` _asbp_player_2))))))
        (:`Completed`
          (set `self.didHit` false))))))

(fn `UserConstructionScript`
  (set `self.weaponParent` (`self.GetParentActor` self)))