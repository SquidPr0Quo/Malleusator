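; BP_GameMode is the game mode for a local multiplayer match in which one randomly chosen player is the monster.
; On BeginPlay it gathers all PlayerStart actors, then creates a local player for each index below MaxPlayerCount with a start tagged with that index.
; It spawns BP_Monster for the random index and BP_Player for the others, possesses each with that player's controller and records them in Players.
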(event `self.ReceiveBeginPlay`
  (`self.GetPlayerStartPoints`)
  (`self.SpawnPlayers`))

(fn `GetPlayerStartPoints`
  (bind _outactors (`GameplayStatics.GetAllActorsOfClass` "/Script/Engine.PlayerStart"))
  (set `self.PlayerStartArray` _outactors))

(fn `SpawnPlayers`
  (bind _index (`self.Index`))
  (bind _players (`self.Players`))
  (bind _maxplayercount (`self.MaxPlayerCount`))
  (bind _returnvalue (`GameplayStatics.GetPlayerController` (`self.Index`)))
  (set `self.MonsterIndex` (`KismetMathLibrary.RandomInteger` _maxplayercount))
  (for _index_2 (range _maxplayercount)
    (set `self.Index` _index_2)
    (for _array_element (`self.PlayerStartArray`)
      (if (== (`PlayerStart.PlayerStartTag` _array_element) (`KismetStringLibrary.Conv_StringToName` (`KismetStringLibrary.Conv_IntToString` _index)))
        (`GameplayStatics.CreatePlayer` (`self.Index`))
        (if (== _index (`self.MonsterIndex`))
          (bind _returnvalue_2 (`self.GetTransform` _array_element))
          (bind _returnvalue_3 (`|SpawnActorFromClass` "/Game/Blueprints/BP_Monster.BP_Monster_C" _returnvalue_2 "AlwaysSpawn" "OverrideRootScale" null null))
          (`Controller.Possess` _returnvalue _returnvalue_3)
          (`KismetArrayLibrary.Array_AddUnique` _players _returnvalue_3)
          (else
            (bind _returnvalue_4 (`|SpawnActorFromClass` "/Game/Blueprints/BP_Player.BP_Player_C" _returnvalue_2 "AlwaysSpawn" "OverrideRootScale" null null))
            (`Controller.Possess` _returnvalue _returnvalue_4)
            (`KismetArrayLibrary.Array_AddUnique` _players _returnvalue_4)))))))

(fn `UserConstructionScript`)